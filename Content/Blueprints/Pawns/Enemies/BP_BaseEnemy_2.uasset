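; BP_BaseEnemy_2 is an enemy that constantly homes in on the player.
; BeginPlay caches the first player's pawn.
; Each tick it moves forward a fixed local offset without sweep, so speed depends on frame rate, and smoothly turns toward that pawn with RInterpTo and a look-at rotation.
; A zero local rotation call has no effect, and the construction script is empty.
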(event EventTick
  (params (DeltaSeconds :type Float%20%28single-precision%29))
  (|CallParentFunction DeltaSeconds)
  (Transformation|AddActorLocalOffset "4.000000, 0, 0" false false)
  (Transformation|AddActorLocalRotation (Math|Rotator|MakeRotator 0.0 0.0 0.0) false false)
  (Transformation|SetActorRotation (Math|Interpolation|RInterpTo (Transformation|GetActorRotation) (Math|Rotator|FindLookatRotation (Transformation|GetActorLocation) (Transformation|GetActorLocation (Variables|Default|GetPlayerPawn))) (Utilities|Time|GetWorldDeltaSeconds) 2.0)))

(event EventBeginPlay
  (|CallParentFunction)
  (Variables|Default|SetPlayerPawn (Game|Player|GetPlayerPawn 0)))

(fn ConstructionScript)